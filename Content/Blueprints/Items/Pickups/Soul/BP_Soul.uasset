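; BP_Soul is a soul pickup actor that slowly sinks toward a hover height above the ground.
; On BeginPlay, a downward object trace sets that height 100 units above the impact point, with debug drawing left on.
; Tick lowers the actor at a constant, frame-rate-independent speed while it is above that height.
; It has no collection logic; the overlap event is an empty, disabled node.
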(event EventBeginPlay
  (bind _returnvalue (Transformation|GetActorLocation))
  (bind _outhit (Collision|LineTraceForObjects _returnvalue (- _returnvalue "0.000000,0.000000,2000.000000") (Variables|Default|GetObjectTypesArray) false 0 "ForDuration" true "(R=1.000000,G=0.000000,B=0.000000,A=1.000000)" "(R=0.000000,G=1.000000,B=0.000000,A=1.000000)" 1e+01))
  (Variables|Default|SetDesiredZ (.z (+ (.ImpactPoint (Collision|BreakHitResult _outhit)) "0.000000,0.000000,100.000000"))))

(event Collision|EventActorBeginOverlap
  (params (OtherActor :type Actor%20Object%20Reference)))

(event EventTick
  (params (DeltaSeconds :type Float%20%28single-precision%29))
  (if (> (.z (Transformation|GetActorLocation)) (Variables|Default|GetDesiredZ))
    (Transformation|AddActorWorldOffset (Math|Vector|MakeVector 0.0 0.0 (* DeltaSeconds -1e+01)))))

(fn ConstructionScript)